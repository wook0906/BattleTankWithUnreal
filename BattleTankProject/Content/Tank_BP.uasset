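; Tank pawn Blueprint that wires player input to a tank's movement, aiming, cameras and health bar widget.
; On BeginPlay it hands the barrel, turret and tracks to the TankAiming and TankMovement components and links itself to the health bar widget.
; Axis inputs drive movement intents and rotate the azimuth gimbal and spring arm with frame-rate-scaled speed.
; Holding SwapCam toggles between third- and first-person cameras; Fire calls TankAiming.
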(event EventBeginPlay
  (Class|TankAimingComponent|Init (Variables|Default|GetTankAiming) (Variables|Default|GetBarrel) (Variables|Default|GetTurret))
  (Class|TankMovementComponent|Init (Variables|Default|GetTankMovement) (Variables|Default|GetLeftTrack) (Variables|Default|GetRightTrack))
  (CallFunction|InitHealthBarWidget))

(event Input|ActionEvents|InputActionSwapCam
  (params (Key :type Key%20Structure :default "AnyKey"))
  (:Pressed
    (Components|Activation|ToggleActive (Variables|Default|GetFPSCamera))
    (Components|Activation|ToggleActive (Variables|Default|GetTPSCamera)))
  (:Released
    (Components|Activation|ToggleActive (Variables|Default|GetTPSCamera))
    (Components|Activation|ToggleActive (Variables|Default|GetFPSCamera))))

(event Input|ActionEvents|InputActionFire
  (params (Key :type Key%20Structure :default "AnyKey"))
  (:Pressed
    (Class|TankAimingComponent|Fire (Variables|Default|GetTankAiming))))

(event Input|AxisEvents|InputAxisTurnRight
  (params (AxisValue :type Float%20%28single-precision%29))
  (Class|TankMovementComponent|IntendTurnRight (Variables|Default|GetTankMovement) AxisValue))

(event Input|AxisEvents|InputAxisAimElevation
  (params (AxisValue :type Float%20%28single-precision%29))
  (Transformation|AddLocalRotation (Variables|Default|GetSpringArm) (Math|Rotator|MakeRotator 0.0 (* (Utilities|Time|GetWorldDeltaSeconds) AxisValue 5e+01) 0.0) false false))

(event Input|AxisEvents|InputAxisAimAzimuth
  (params (AxisValue :type Float%20%28single-precision%29))
  (Transformation|AddLocalRotation (Variables|Default|GetAzimuthGimbal) (Math|Rotator|MakeRotator 0.0 0.0 (* (Utilities|Time|GetWorldDeltaSeconds) AxisValue 1e+02)) false false))

(event Input|AxisEvents|InputAxisMoveForward
  (params (AxisValue :type Float%20%28single-precision%29))
  (Class|TankMovementComponent|IntendMoveForward (Variables|Default|GetTankMovement) AxisValue))

(fn ConstructionScript)

(fn InitHealthBarWidget
  (bind _asheath_bar_bp (Utilities|Casting|CastToHeathBar_BP (UserInterface|GetUserWidgetObject (Variables|Default|GetHealthBar)))
    (:then
      (Variables|/Game/HeathBar_BP.HeathBar_BP_C|SetMyTank _asheath_bar_bp self))
    (:CastFailed
      _))
  (return))